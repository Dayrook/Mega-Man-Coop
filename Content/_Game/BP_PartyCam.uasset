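; BP_PartyCam is a party camera actor that follows the group of BP_mm_Player characters along the X axis.
; A self-repeating event refreshes the player list twice a second.
; Each Tick, DetermineTargetPosition takes the midpoint of the leftmost and rightmost valid players' capsule positions.
; The scene component snaps to that X without smoothing, keeping a fixed Y and the CameraHeight Z.
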(event Custom|CountPlayers
  (bind _outactors (Actor|GetAllActorsOfClass "/Game/_Player/BP_mm_Player.BP_mm_Player_C"))
  (Variables|Default|SetPlayers _outactors)
  (Utilities|FlowControl|Delay 0.5)
  (CallFunction|CountPlayers))

(event EventBeginPlay
  (CallFunction|CountPlayers))

(event Collision|EventActorBeginOverlap
  (params (OtherActor :type Actor%20Object%20Reference)))

(event EventTick
  (params (DeltaSeconds :type Float%20%28single-precision%29))
  (Transformation|SetWorldLocation (Variables|Default|GetSceneComponent) (Math|Vector|MakeVector (CallFunction|DetermineTargetPosition) 1e+02 (Variables|Default|GetCameraHeight)) false false))

(fn ConstructionScript)

(fn DetermineTargetPosition
  (for _array_element (Variables|Default|GetPlayers)
    (Utilities|IsValid _array_element
      (:Is%20Valid
        (Utilities|FlowControl|Sequence
          (:then_0
            (if (<= (.x (Transformation|GetWorldLocation (Variables|/Script/Engine.Character|GetCapsuleComponent _array_element))) (LocalVariables|GetLeftMost))
              (LocalVariables|SetLeftMost (.x (Transformation|GetWorldLocation (Variables|/Script/Engine.Character|GetCapsuleComponent _array_element))))))
          (:then_1
            (if (>= (.x (Transformation|GetWorldLocation (Variables|/Script/Engine.Character|GetCapsuleComponent _array_element))) (LocalVariables|GetRightMost))
              (LocalVariables|SetRightMost (.x (Transformation|GetWorldLocation (Variables|/Script/Engine.Character|GetCapsuleComponent _array_element))))))))))
  (bind _output_get (LocalVariables|SetAverageX (/ (+ (LocalVariables|GetRightMost) (LocalVariables|GetLeftMost)) 2.0)))
  (return _output_get))