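; BP_Shooter is a 2D flipbook enemy that repeatedly fires projectiles in the direction it faces.
; After an initial interval, ShootSomething turns it toward the player, plays a non-looping wind-up flipbook, then spawns MyProjectile at a facing-based offset with a signed speed.
; It restores the looping idle flipbook and calls itself again after ShootInterval, forming a delay-driven attack loop without Tick.
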(event Custom|ShootSomething
  (bind _returnvalue (Transformation|GetActorTransform))
  (bind _sprite (Variables|Default|GetSprite))
  (CallFunction|FacePlayer)
  (Utilities|FlowControl|Delay 0.2)
  (Sprite|SetFlipbook _sprite (Variables|Default|GetWindUpFlipbook))
  (Components|Timeline|SetLooping _sprite false)
  (Utilities|FlowControl|Delay (Variables|Default|GetWindUpInterval))
  (bind _returnvalue_2 (Game|SpawnActorfromClass (Variables|Default|GetMyProjectile) (Math|Transform|MakeTransform (+ (.location _returnvalue) (Math|Vector|MakeVector (Utilities|Select :Index (Variables|Default|GetFacing) :NewEnumerator0 1e+01 :NewEnumerator1 -1e+01) 1e+01 -12.0)) (.rotation _returnvalue) (.scale _returnvalue)) "Undefined" 0 0))
  (Variables|/Game/_Enemies/Shooters/BP_EnemyBullet.BP_EnemyBullet_C|SetSpeed _returnvalue_2 (Utilities|Select :Index (Variables|Default|GetFacing) :NewEnumerator0 8e+01 :NewEnumerator1 -8e+01))
  (Sprite|SetFlipbook (Variables|Default|GetSprite) (Variables|Default|GetIdleFlipbook))
  (Components|Timeline|SetLooping (Variables|Default|GetSprite) true)
  (Audio|Components|Audio|Play (Variables|Default|GetSprite))
  (Utilities|FlowControl|Delay (Variables|Default|GetShootInterval))
  (CallFunction|ShootSomething))

(event EventBeginPlay
  (|CallParentFunction)
  (Utilities|FlowControl|Delay (Variables|Default|GetShootInterval))
  (CallFunction|ShootSomething))

(event Collision|EventActorBeginOverlap
  (params (OtherActor :type Actor%20Object%20Reference))
  (|CallParentFunction OtherActor) ; This node is disabled and will not be called.\nDrag off pins to build functionality.
)

(event EventTick
  (params (DeltaSeconds :type Float%20%28single-precision%29))
  (|CallParentFunction DeltaSeconds) ; This node is disabled and will not be called.\nDrag off pins to build functionality.
)

(fn ConstructionScript
  (|CallParentFunction))