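; BP_EnemyBullet is a projectile actor for shooter enemies that plays a 2D sound when it spawns.
; Each tick it moves along its local X axis by Speed scaled by delta time, using a plain offset rather than a movement component.
; On overlapping a valid actor it stores that actor as HitActor and destroys itself, unless the actor carries the IgnoreEnemyBullet tag.
; The graph itself applies no damage.
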(event EventBeginPlay
  (Audio|PlaySound2D (Variables|Default|GetSoundOnSpawn) 0.6 1.0 0.0 0 0))

(event Collision|EventActorBeginOverlap
  (params (OtherActor :type Actor%20Object%20Reference))
  ;[1 1 1] Destruction
  (if (Utilities|IsValid OtherActor)
    (bind _output_get (Variables|Default|SetHitActor OtherActor))
    (if (not (Utilities|Array|ContainsItem (Variables|/Script/Engine.Actor|GetTags _output_get) "IgnoreEnemyBullet"))
      ;[1 1 1] Remove Bullet Actor
      (Actor|DestroyActor))))

(event EventTick
  (params (DeltaSeconds :type Float%20%28single-precision%29))
  (Transformation|AddActorLocalOffset (Math|Vector|MakeVector (* (Variables|Default|GetSpeed) 1.0 (Utilities|Time|GetWorldDeltaSeconds)) 0.0 0.0) false false))

(fn ConstructionScript)