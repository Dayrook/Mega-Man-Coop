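; BP_MetBulldozer is a bulldozer Met enemy that rolls horizontally at a constant speed.
; On BeginPlay it sets its health, waits briefly, then picks a direction once toward the target player's X position, rotating the sprite when heading positive X.
; Tick then moves the capsule by setting its world location directly, scaled by delta time.
; Movement-component, velocity and AI move attempts remain as unconnected leftovers.
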(event EventBeginPlay
  (|CallParentFunction)
  (Variables|Default|SetHealth 1.1e+02)
  (Utilities|FlowControl|Delay 0.5)
  (if (<= (- (.x (Transformation|GetWorldLocation (Variables|/Script/Paper2D.PaperCharacter|GetSprite (Variables|Default|GetMyTargetPlayer)))) (.x (Transformation|GetWorldLocation (Variables|Default|GetCapsuleComponent)))) 0.0)
    (Variables|Default|SetSpeed -2e+01)
    (else
      (Variables|Default|SetSpeed 2e+01)
      (Transformation|SetRelativeRotation (Variables|Default|GetSprite) "0,180.000000, 0" false false)))
  (Variables|Default|SetMoveItOut true))

(event Collision|EventActorBeginOverlap
  (params (OtherActor :type Actor%20Object%20Reference))
  (|CallParentFunction OtherActor) ; This node is disabled and will not be called.\nDrag off pins to build functionality.
)

(event EventTick
  (params (DeltaSeconds :type Float%20%28single-precision%29))
  (bind _capsulecomponent (Variables|Default|GetCapsuleComponent))
  (bind _returnvalue (Transformation|GetWorldLocation _capsulecomponent))
  (|CallParentFunction DeltaSeconds)
  (if (Variables|Default|GetMoveItOut)
    (Transformation|SetWorldLocation (Variables|Default|GetCapsuleComponent) (Math|Vector|MakeVector (+ (* DeltaSeconds (Variables|Default|GetSpeed)) (.x _returnvalue)) (.y _returnvalue) (.z _returnvalue)) false false)))

(fn ConstructionScript
  (|CallParentFunction))