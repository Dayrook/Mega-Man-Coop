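; BP_SimpleSPawn is an enemy spawner that creates a SpawnThis instance when a BP_mm_Player overlaps it.
; One second after BeginPlay it sizes its Box from the game mode's ScreenWidth.
; Each player overlap spawns at the PaperSprite's transform, lifts the enemy by its capsule half-height and sets that player as its target.
; Nothing limits repeat spawns, and a failed spawn prints the class name.
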(event EventBeginPlay
  (Utilities|FlowControl|Delay 1.0)
  (bind _asmm_game_mode (Utilities|Casting|CastTomm_GameMode (Game|GetGameMode)))
  (Components|Box|SetBoxExtent (Variables|Default|GetBox) (Math|Vector|MakeVector (Variables|/Game/_Game/mm_GameMode.mm_GameMode_C|GetScreenWidth _asmm_game_mode) 5e+01 (Variables|/Game/_Game/mm_GameMode.mm_GameMode_C|GetScreenWidth _asmm_game_mode)) true))

(event Collision|EventActorBeginOverlap
  (params (OtherActor :type Actor%20Object%20Reference))
  (bind _spawnthis (Variables|Default|GetSpawnThis))
  (bind _papersprite (Variables|Default|GetPaperSprite))
  (bind _returnvalue (Transformation|GetWorldTransform _papersprite))
  (bind _asbp_mm_player (Utilities|Casting|CastToBP_mm_Player OtherActor))
  (Variables|Default|SetPlayerAggroed _asbp_mm_player)
  (bind _returnvalue_2 (Game|SpawnActorfromClass _spawnthis (Transformation|GetWorldTransform (Variables|Default|GetPaperSprite)) "AdjustIfPossibleButAlwaysSpawn" 0 0))
  (Utilities|IsValid _returnvalue_2
    (:Is%20Valid
      (Variables|Default|SetSpawnedEnemy _returnvalue_2)
      (Transformation|SetWorldLocation (Variables|/Script/Engine.Actor|GetRootComponent (Variables|Default|GetSpawnedEnemy)) (Math|Vector|MakeVector (.x (.location _returnvalue)) (.y (.location _returnvalue)) (+ (.z (.location _returnvalue)) (Variables|/Script/Engine.CapsuleComponent|GetCapsuleHalfHeight (Variables|/Script/Engine.Character|GetCapsuleComponent _returnvalue_2)))) false false)
      (Variables|/Game/_Enemies/BP_EnemyBase.BP_EnemyBase_C|SetMyTargetPlayer (Variables|Default|GetSpawnedEnemy) (Variables|Default|GetPlayerAggroed)))
    (:Is%20Not%20Valid
      (Development|PrintString (Utilities|String|Append "Failed Spawn : " (Utilities|GetClassDisplayName _spawnthis))))))

(event EventTick
  (params (DeltaSeconds :type Float%20%28single-precision%29)))

(fn ConstructionScript)