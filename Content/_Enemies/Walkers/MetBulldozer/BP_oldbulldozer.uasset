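; Older-named Met Bulldozer walker enemy that trundles horizontally in the direction of the player's position shortly after spawning.
; BeginPlay sets health, then after a short delay compares X positions with the target player to pick a signed walk speed, flipping the sprite for rightward travel.
; Tick then moves it through the CharacterMovement component at that constant speed, scaled by delta time, without re-targeting.
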(event EventBeginPlay
  (|CallParentFunction)
  (Variables|Default|SetHealth 1.1e+02)
  (Utilities|FlowControl|Delay 0.5)
  (if (<= (- (.x (Transformation|GetWorldLocation (Variables|/Script/Paper2D.PaperCharacter|GetSprite (Variables|Default|GetMyTargetPlayer)))) (.x (Transformation|GetWorldLocation (Variables|Default|GetCapsuleComponent)))) 0.0)
    (Variables|Default|SetWalkSpeed -2e+01)
    (else
      (Variables|Default|SetWalkSpeed 2e+01)
      (CallFunction|SetSpriteFaceDirection "NewEnumerator1")))
  ;[1 1 1] Comment
  (Variables|Default|SetMoveItOut true))

(event Collision|EventActorBeginOverlap
  (params (OtherActor :type Actor%20Object%20Reference))
  (|CallParentFunction OtherActor) ; This node is disabled and will not be called.\nDrag off pins to build functionality.
)

(event EventTick
  (params (DeltaSeconds :type Float%20%28single-precision%29))
  (|CallParentFunction DeltaSeconds)
  (if (Variables|Default|GetMoveItOut)
    (Class|MovementComponent|MoveUpdatedComponent (Variables|Character|GetCharacterMovement) (Math|Vector|MakeVector (* DeltaSeconds (Variables|Default|GetWalkSpeed)) 0.0 0.0) "0, 0, 0" true)))

(fn ConstructionScript
  (|CallParentFunction))