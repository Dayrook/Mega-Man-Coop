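; BP_EnemyBase is an enemy base Blueprint that provides shared health and death handling.
; Its TakeDamage event subtracts the damage amount from Health and calls Die once Health reaches zero or below.
; Die spawns a separate BP_DeathAnim actor at the capsule's world transform, then destroys the enemy.
; BeginPlay, Tick and the construction script are empty.
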(event Custom|TakeDamage
  (params (DmgAmount :type Float%20%28single-precision%29))
  (bind _output_get (Variables|Default|SetHealth (- (Variables|Default|GetHealth) DmgAmount)))
  (if (<= _output_get 0.0)
    (CallFunction|Die)))

(event Custom|Die
  (Game|SpawnActorfromClass "/Game/_Enemies/Death/BP_DeathAnim.BP_DeathAnim_C" (Transformation|GetWorldTransform (Variables|Collision|GetCapsuleComponent)) "Undefined" 0 0)
  (Actor|DestroyActor))

(event EventBeginPlay)

(event Collision|EventActorBeginOverlap
  (params (OtherActor :type Actor%20Object%20Reference)))

(event EventTick
  (params (DeltaSeconds :type Float%20%28single-precision%29)))

(fn ConstructionScript)