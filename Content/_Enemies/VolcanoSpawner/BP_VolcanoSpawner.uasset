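; Paper2D volcano enemy spawner that rises when the player enters its sphere, then launches enemies upward.
; Timelines move the flipbook up and down while flipbook swaps show each state.
; A delayed self-calling SpawnEnemy asks mm_GameMode for permission and impulses each spawn with random sideways drift.
; A refusal or reached quota makes it dormant; with LoopSpawning it submerges and resets for another trigger.
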(event OnComponentBeginOverlap(Sphere)
  (params (OverlappedComponent :type Primitive%20Component%20Object%20Reference) (OtherActor :type Actor%20Object%20Reference) (OtherComp :type Primitive%20Component%20Object%20Reference) (OtherBodyIndex :type Integer) (bFromSweep :type Boolean) (SweepResult :type Hit%20Result%20Structure%20%28by%20ref%29))
  ;[1 1 1] Should Emerge?
  (if (not (Variables|Default|GetEmerged))
    (if (== (Utilities|GetClass OtherActor) "/Game/_Player/BP_mm_Player.BP_mm_Player_C")
      (Variables|Default|SetEmerged true)
      ;[1 1 1] Emerge
      (bind _level (Timeline|EmergeTL PlayFromStart)
        (:Update
          (Transformation|SetRelativeLocation (Variables|Default|GetPaperFlipbook) (Math|Vector|MakeVector 0.0 (Variables|Default|GetFlipbookYDepth) (Math|Float|Lerp -6.0 1e+01 _level)) false false))
        (:Finished
          ;[1 1 1] Start Spawning
          (Sprite|SetFlipbook (Variables|Default|GetPaperFlipbook) "/Game/_Enemies/VolcanoSpawner/Animation/FB_Volcano2.FB_Volcano2")
          (Utilities|FlowControl|Delay (Variables|Default|GetSpawnInterval))
          (Sprite|SetFlipbook (Variables|Default|GetPaperFlipbook) "/Game/_Enemies/VolcanoSpawner/Animation/FB_Volcano3.FB_Volcano3")
          (CallFunction|SpawnEnemy))))))

(event Custom|SpawnEnemy
  (bind _scene (Variables|Default|GetScene))
  (bind _returnvalue (Transformation|GetWorldTransform _scene))
  ;[1 1 1] If OK to Spawn
  (bind _asmm_game_mode (Utilities|Casting|CastTomm_GameMode (Game|GetGameMode))
    (:then
      (if (< (Variables|Default|GetSpawnedEnemyCount) (Variables|Default|GetNumberToSpawn))
        (bind _permitspawn (Default|RequestEnemySpawn _asmm_game_mode))
        (if _permitspawn
          ;[1 1 1] Spawn with Impulse
          (bind _returnvalue_2 (Game|SpawnActorfromClass (Variables|Default|GetEnemyType) (Math|Transform|MakeTransform (+ (.location _returnvalue) "0,0.000000,16.000000") (.rotation _returnvalue) (.scale _returnvalue)) "Undefined" 0 0 :!label _label))
          (Utilities|IsValid _returnvalue_2
            (:Is%20Valid
              (Physics|AddImpulse (Variables|/Script/Engine.Character|GetCapsuleComponent _returnvalue_2) (* (Math|Vector|MakeVector (Math|Random|RandomFloatinRange -0.2 0.2) 0.0 1.0) (* (Variables|Default|GetLaunchImpulse) 1e+04)) "None" false)
              (Math|Integer|IncrementInt (Variables|Default|GetSpawnedEnemyCount)
                (:%20%20
                  _)))
            (:Is%20Not%20Valid
              _))
          (Utilities|FlowControl|Delay (Variables|Default|GetSpawnInterval))
          (CallFunction|SpawnEnemy)
          (else
            ;[1 1 1] Go Dormant
            (CallFunction|BecomeDormant :!label _label_2)))
        (else
          (goto _label_2))))
    (:CastFailed
      (Development|PrintString "Incorrect Game Mode")
      (goto _label))))

(event Custom|BecomeDormant
  (Sprite|SetFlipbook (Variables|Default|GetPaperFlipbook) "/Game/_Enemies/VolcanoSpawner/Animation/FB_Volcano4.FB_Volcano4")
  (if (Variables|Default|GetLoopSpawning)
    (bind _submergelevel (Timeline|SubmergeTL PlayFromStart)
      (:Update
        (Transformation|SetRelativeLocation (Variables|Default|GetPaperFlipbook) (Math|Vector|MakeVector 0.0 (Variables|Default|GetFlipbookYDepth) (Math|Float|Lerp 1e+01 -6.0 _submergelevel)) false false))
      (:Finished
        ;[1 1 1] Reset to Spawn Again
        (Variables|Default|SetEmerged false)
        (Variables|Default|SetSpawnedEnemyCount 0)
        (Sprite|SetFlipbook (Variables|Default|GetPaperFlipbook) "/Game/_Enemies/VolcanoSpawner/Animation/FB_Volcano1.FB_Volcano1")))))

(event EventBeginPlay
  (Transformation|SetRelativeLocation (Variables|Default|GetPaperFlipbook) "0, 0,-6.000000" false false))

(event EventTick
  (params (DeltaSeconds :type Float%20%28single-precision%29)))

(fn ConstructionScript)