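; BP_EyeWalker is a walking enemy that moves horizontally toward its target player.
; After a short startup delay, a self-recalling event compares X positions every half second to flip walk speed and facing, with the facing enum noted as reversed.
; Tick moves the movement component along X by that speed scaled by delta time.
; Health is set after the first tracking call, and facing comes from inherited logic.
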(event Custom|MoveTargetTowardPlayer
  (if (<= (- (.x (Transformation|GetWorldLocation (Variables|/Script/Paper2D.PaperCharacter|GetSprite (Variables|Default|GetMyTargetPlayer)))) (.x (Transformation|GetWorldLocation (Variables|Default|GetCapsuleComponent)))) 0.0)
    (Variables|Default|SetWalkSpeed -1e+01)
    ;[1 1 1] reversed from normal
    (CallFunction|SetFacingDirection "NewEnumerator1")
    (else
      (Variables|Default|SetWalkSpeed 1e+01)
      (CallFunction|SetFacingDirection "NewEnumerator0")))
  (Utilities|FlowControl|Delay 0.5)
  (CallFunction|MoveTargetTowardPlayer))

(event EventBeginPlay
  (|CallParentFunction)
  (Utilities|FlowControl|Delay 0.2)
  (CallFunction|MoveTargetTowardPlayer)
  (Variables|Default|SetHealth 5.0))

(event Collision|EventActorBeginOverlap
  (params (OtherActor :type Actor%20Object%20Reference))
  (|CallParentFunction OtherActor) ; This node is disabled and will not be called.\nDrag off pins to build functionality.
)

(event EventTick
  (params (DeltaSeconds :type Float%20%28single-precision%29))
  (|CallParentFunction DeltaSeconds)
  (Class|MovementComponent|MoveUpdatedComponent (Variables|Character|GetCharacterMovement) (Math|Vector|MakeVector (* DeltaSeconds (Variables|Default|GetWalkSpeed)) 0.0 0.0) "0, 0, 0" true))

(fn ConstructionScript
  (|CallParentFunction))