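; BP_VictoryPickup is a pickup that triggers map victory when the player touches it.
; On BeginPlay it sets the pickup sound to a crystal effect.
; On overlap it runs the parent's logic, then, if the other actor's class is exactly BP_mm_Player, casts the game mode to mm_GameMode and calls MapVictory.
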(event EventBeginPlay
  (|CallParentFunction)
  (Variables|Default|SetSoundOnPickup "/Game/_Audio/mm2_sfx_crystal.mm2_sfx_crystal"))

(event Collision|EventActorBeginOverlap
  (params (OtherActor :type Actor%20Object%20Reference))
  (|CallParentFunction OtherActor)
  (if (== (Utilities|GetClass OtherActor) "/Game/_Player/BP_mm_Player.BP_mm_Player_C")
    (bind _asmm_game_mode (Utilities|Casting|CastTomm_GameMode (Game|GetGameMode)))
    (Default|MapVictory _asmm_game_mode)))

(event EventTick
  (params (DeltaSeconds :type Float%20%28single-precision%29))
  (|CallParentFunction DeltaSeconds) ; This node is disabled and will not be called.\nDrag off pins to build functionality.
)

(fn ConstructionScript
  (|CallParentFunction))