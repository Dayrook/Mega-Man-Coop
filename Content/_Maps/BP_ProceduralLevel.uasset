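; Level builder actor that procedurally lays out a horizontal Paper2D tilemap level at BeginPlay.
; It spawns a set number of mid-segment tilemaps end to end along X from a placed start tilemap, each with an obstacle at its horizontal center.
; It then caps the run with an end tilemap and a victory pickup.
; Spawn positions derive from segment count and tile dimensions.
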(event Custom|BuildSegmentsAndObstacles
  (bind _tiledimension (Variables|Default|GetTileDimension))
  (bind _tiledimension_2 (Variables|Default|GetTileDimension))
  (while (< (Variables|Default|GetSegmentsBuilt) (Variables|Default|GetSegmentsToBuild))
    (bind _returnvalue (Game|SpawnActorfromClass "/Script/Paper2D.PaperTileMapActor" (Math|Transform|MakeTransform (CallFunction|CalcSegmentPosition) "0, 0, 0" "1,1,1") "Undefined" 0 0))
    (Class|PaperTileMapComponent|SetTileMap (Variables|/Script/Paper2D.PaperTileMapActor|GetRenderComponent _returnvalue) "/Game/_Maps/_Tiles/Mid_Tilemap.Mid_Tilemap")
    (Math|Integer|IncrementInt (Variables|Default|GetSegmentsBuilt)
      (:%20%20
        (Game|SpawnActorfromClass "/Game/_Maps/Obstacles/BP_Obstacle.BP_Obstacle_C" (Math|Transform|MakeTransform (+ (Variables|Default|GetCurrentSegmentPosition) (Math|Vector|MakeVector (* (* (Variables|Default|GetXTilesInSegment) _tiledimension_2) 0.5) 0.0 (* (Math|Conversions|ToFloat(Integer) (* _tiledimension_2 (- (Variables|Default|GetYTilesInSegment) 9))) -1.0))) "0, 0, 0" "1,1,1") "AdjustIfPossibleButAlwaysSpawn" 0 0))))
  (bind _returnvalue_2 (Game|SpawnActorfromClass "/Script/Paper2D.PaperTileMapActor" (Math|Transform|MakeTransform (CallFunction|CalcSegmentPosition) "0, 0, 0" "1,1,1") "Undefined" 0 0))
  (Class|PaperTileMapComponent|SetTileMap (Variables|/Script/Paper2D.PaperTileMapActor|GetRenderComponent _returnvalue_2) "/Game/_Maps/_Tiles/End_Tilemap.End_Tilemap")
  (Game|SpawnActorfromClass "/Game/_Items/BP_VictoryPickup.BP_VictoryPickup_C" (Math|Transform|MakeTransform (+ (Variables|Default|GetCurrentSegmentPosition) (Math|Vector|MakeVector (* (* (Variables|Default|GetXTilesInSegment) _tiledimension) 0.2) 0.0 (* (Math|Conversions|ToFloat(Integer) (* _tiledimension (- (Variables|Default|GetYTilesInSegment) 9))) -1.0))) "0, 0, 0" "1,1,1") "Undefined" 0 0))

(event EventBeginPlay
  (CallFunction|BuildSegmentsandObstacles))

(event Collision|EventActorBeginOverlap
  (params (OtherActor :type Actor%20Object%20Reference)))

(event EventTick
  (params (DeltaSeconds :type Float%20%28single-precision%29)))

(fn ConstructionScript)

(fn CalcSegmentPosition
  (bind _starttilemap (Variables|Default|GetStartTileMap))
  (bind _returnvalue (Transformation|GetWorldLocation _starttilemap))
  (bind _output_get (Variables|Default|SetCurrentSegmentPosition (Math|Vector|MakeVector (+ (Math|Conversions|ToFloat(Integer) (* (Variables|Default|GetTileDimension) (Variables|Default|GetXTilesInSegment) (Variables|Default|GetSegmentsBuilt))) (.x _returnvalue)) 0.0 (.z _returnvalue))))
  (return _output_get))