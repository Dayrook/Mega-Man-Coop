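; BP_Obstacle is a level obstacle that randomizes its platform layout and the enemy it spawns.
; On BeginPlay it picks one of three enemy classes and a tilemap option, offsetting the geometry to suit.
; After a short delay it usually creates a BP_SimpleSpawn for that enemy.
; Rarely, it instead clears the tilemap and places a BP_VolcanoSpawner at a randomized height, passing it the same enemy type.
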(event Custom|GenerateParams
  ;[1 1 1] Choose Enemy to Spawn
  (bind _output_get (Variables|Default|SetRando1 (Math|Random|RandomIntegerinRange 0 2)))
  (Variables|Default|SetEnemyType (Utilities|Select :Index _output_get :Option%200 "/Game/_Enemies/BP_EnemyBase.BP_EnemyBase_C" :Option%201 "/Game/_Enemies/EyeWalker/BP_EyeWalker.BP_EyeWalker_C" :Option%202 "/Game/_Enemies/MetBulldozer/BP_MetBulldozer.BP_MetBulldozer_C"))
  ;[1 1 1] Choose Tileset
  (Variables|Default|SetRando2 (Math|Random|RandomIntegerinRange 0 3))
  (Class|PaperTileMapComponent|SetTileMap (Variables|Default|GetObstacleGeometry) (Utilities|Select :Index (Variables|Default|GetRando2) :Option%200 0 :Option%201 "/Game/_Maps/_Tiles/Obs_3x2_Tilemap.Obs_3x2_Tilemap" :Option%202 "/Game/_Maps/_Tiles/Obs_5x1_Tilemap.Obs_5x1_Tilemap" :Option%203 "/Game/_Maps/_Tiles/Obs_Stair_Platform.Obs_Stair_Platform"))
  (Transformation|SetRelativeLocation (Variables|Default|GetObstacleGeometry) (Math|Vector|MakeVector (Math|Conversions|ToFloat(Integer) (Math|Random|RandomIntegerinRange -30 10)) 0.0 (Utilities|Select :Index (Variables|Default|GetRando2) :Option%200 0.0 :Option%201 16.0 :Option%202 0.0 :Option%203 48.0)) false false))

(event EventBeginPlay
  (bind _spawnerlocation1 (Variables|Default|GetSpawnerLocation1))
  (bind _returnvalue (Transformation|GetWorldLocation _spawnerlocation1))
  (CallFunction|GenerateParams)
  (Utilities|FlowControl|Delay 0.2)
  (if (Math|Random|RandomBoolwithWeight 0.9)
    ;[1 1 1] Create Enemy Spawner
    (bind _returnvalue_2 (Game|SpawnActorfromClass "/Game/_Enemies/SimpleSpawn/BP_SimpleSPawn.BP_SimpleSpawn_C" (Math|Transform|MakeTransform (Transformation|GetWorldLocation (Variables|Default|GetSpawnerLocation1)) "0, 0, 0" "1,1,1") "AdjustIfPossibleButAlwaysSpawn" 0 0))
    (Utilities|IsValid _returnvalue_2
      (:Is%20Valid
        (bind _output_get (Variables|Default|SetSimpleSpawner _returnvalue_2))
        (Variables|/Game/_Enemies/SimpleSpawn/BP_SimpleSPawn.BP_SimpleSpawn_C|SetSpawnThis _output_get (Variables|Default|GetEnemyType)))
      (:Is%20Not%20Valid
        (Development|PrintString "Invalid Spawner")))
    (else
      (Class|PaperTileMapComponent|SetTileMap (Variables|Default|GetObstacleGeometry))
      (bind _returnvalue_3 (Game|SpawnActorfromClass "/Game/_Enemies/VolcanoSpawner/BP_VolcanoSpawner.BP_VolcanoSpawner_C" (Math|Transform|MakeTransform (Math|Vector|MakeVector (.x _returnvalue) 0.0 (+ (.z _returnvalue) (Math|Random|RandomFloatinRange -32.0 16.0))) "0, 0, 0" "1,1,1") "Undefined" 0 0))
      (Variables|/Game/_Enemies/VolcanoSpawner/BP_VolcanoSpawner.BP_VolcanoSpawner_C|SetEnemyType _returnvalue_3 (Variables|Default|GetEnemyType)))))

(event Collision|EventActorBeginOverlap
  (params (OtherActor :type Actor%20Object%20Reference)))

(event EventTick
  (params (DeltaSeconds :type Float%20%28single-precision%29)))

(fn ConstructionScript)