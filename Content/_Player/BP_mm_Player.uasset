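; Side-scrolling 2D player character with running, jumping, shooting, enemy-hit reactions and input to add or remove players.
; Tick derives a state from speed, air and shooting flags, turns the controller to face travel, and picks the matching flipbook, carrying playback position into run animations.
; Shoot spawns a bullet with a brief shooting pose.
; An enemy hit locks control, forces horizontal movement and grants temporary invulnerability.
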(event Custom|HandleDamage
  ;[1 1 1] Damaged State : Enter and Exit
  (Variables|Default|SetIsInvulnerable true)
  (Variables|Default|SetState "NewEnumerator5")
  (Utilities|FlowControl|Delay 1.0)
  (Variables|Default|SetState "NewEnumerator0")
  (Utilities|FlowControl|Delay 1.0)
  (Variables|Default|SetIsInvulnerable false))

(event Custom|UpdateAnimation
  ;[1 1 1] Set Animation Flipbook
  (|SwitchonStateforAnimation))

(event EventOnLanded
  (params (Hit :type Hit%20Result%20Structure%20%28by%20ref%29))
  ;[1 1 1] Handle Jump
  (Variables|Default|SetIsInAir false))

(event EventTick
  (params (DeltaSeconds :type Float%20%28single-precision%29))
  ;[1 1 1] Tick - Determines animation
  (Variables|Default|SetSpeed (Math|Vector|VectorLength (Transformation|GetVelocity)))
  (CallFunction|UpdateAnimation)
  (if (Utilities|Enum|Equal(Enum) (Variables|Default|GetState) "NewEnumerator5")
    (Pawn|Input|AddMovementInput "1.000000, 0, 0" (Utilities|Select :Index (Variables|Default|GetFacingDirection) :NewEnumerator0 -0.8 :NewEnumerator1 0.8) false) ; Damage Movement
    (else
      (Math|Float|CompareFloat (.X (Math|Vector|BreakVector (Variables|/Script/Engine.MovementComponent|GetVelocity (Pawn|GetMovementComponent)))) 0.0
        (:>
          (Pawn|SetControlRotation (Pawn|GetController) (Math|Rotator|MakeRotator 0.0 0.0 0.0) :!label _label))
        (:==
          (if (Variables|Default|GetIsMovingRight)
            (goto _label)
            (else
              (Pawn|SetControlRotation (Pawn|GetController) (Math|Rotator|MakeRotator 0.0 0.0 1.8e+02) :!label _label_2))))
        (:<
          (goto _label_2)))
      (if (Variables|Default|GetIsInAir)
        (if (Variables|Default|GetIsShooting)
          (Variables|Default|SetState "NewEnumerator4")
          (else
            (Variables|Default|SetState "NewEnumerator3")))
        (elif (> (Variables|Default|GetSpeed) 5e+01)
          (if (Variables|Default|GetIsShooting)
            (Variables|Default|SetState "NewEnumerator8")
            (else
              (Variables|Default|SetState "NewEnumerator7")))
          (elif (Variables|Default|GetIsShooting)
            (Variables|Default|SetState "NewEnumerator2")
            (elif (> (Variables|Default|GetSpeed) 1.0)
              (Variables|Default|SetState "NewEnumerator1")
              (else
                (Variables|Default|SetState "NewEnumerator0")))))))))

(event Collision|EventHit
  (params (MyComp :type Primitive%20Component%20Object%20Reference) (Other :type Actor%20Object%20Reference) (OtherComp :type Primitive%20Component%20Object%20Reference) (bSelfMoved :type Boolean) (HitLocation :type Vector :default "0, 0, 0") (HitNormal :type Vector :default "0, 0, 0") (NormalImpulse :type Vector :default "0, 0, 0") (Hit :type Hit%20Result%20Structure%20%28by%20ref%29))
  ;[1 1 1] Overlapping Thing That Hurts Me
  (if (not (Variables|Default|GetIsInvulnerable))
    (if (Utilities|Array|ContainsItem (Utilities|Array|MakeArray "/Game/_Enemies/BP_EnemyBase.BP_EnemyBase_C") (Utilities|GetClass Other))
      (CallFunction|HandleDamage))))

(event EventBeginPlay
  (Class|CameraComponent|SetOrthoWidth (Variables|Camera|GetSideViewCameraComponent) 255.0)
  (Class|ActorComponent|SetIsReplicated (Variables|Default|GetSprite) true)
  (Variables|Default|SetJumpMaxHoldTime 0.2)
  (bind _asmm_game_mode (Utilities|Casting|CastTomm_GameMode (Game|GetGameMode)))
  (Variables|/Game/_Game/mm_GameMode.mm_GameMode_C|SetScreenWidth _asmm_game_mode (Variables|/Script/Engine.CameraComponent|GetOrthoWidth (Variables|Camera|GetSideViewCameraComponent))))

(event Input|ActionEvents|InputActionShoot
  (params (Key :type Key%20Structure))
  (bind _returnvalue (Transformation|GetActorTransform))
  ;[1 1 1] Attack
  (:Pressed
    (if (Utilities|Enum|NotEqual(Enum) (Variables|Default|GetState) "NewEnumerator5")
      (Variables|Default|SetIsShooting true)
      (Game|SpawnActorfromClass "/Game/_Player/_Attack/BP_Bullet_Base.BP_Bullet_Base_C" (Math|Transform|MakeTransform (+ (.location _returnvalue) (Math|Vector|MakeVector (select (Variables|Default|GetIsMovingRight) 8.0 -8.0) 0.0 0.0)) (.rotation _returnvalue) (.scale _returnvalue)) "Undefined" 0 0)
      (Utilities|FlowControl|Delay 0.2)
      (Variables|Default|SetIsShooting false))))

(event Input|ActionEvents|InputActionQuitGameButton
  (params (Key :type Key%20Structure))
  ;[1 1 1] Quit Game
  (:Pressed
    (Game|QuitGame 0 "Quit" false)))

(event Input|ActionEvents|InputActionAddPlayer
  (params (Key :type Key%20Structure))
  ;[1 1 1] Add / Remove Players
  (:Pressed
    (Default|CallAddPlayerDispatch)))

(event Input|ActionEvents|InputActionRemovePlayer
  (params (Key :type Key%20Structure))
  ;[1 1 1] Add / Remove Players
  (:Pressed
    (Default|CallRemovePlayerDispatch)))

(event Input|ActionEvents|InputActionJump
  (params (Key :type Key%20Structure))
  ;[1 1 1] Handle Jump
  (:Pressed
    (if (Utilities|Enum|NotEqual(Enum) (Variables|Default|GetState) "NewEnumerator5")
      (Character|Jump)
      (Variables|Default|SetIsInAir true)))
  (:Released
    (Character|StopJumping)))

(event Input|AxisEvents|InputAxisMoveRight
  (params (AxisValue :type Float%20%28single-precision%29))
  ;[1 1 1] Handle movement
  (if (Utilities|Enum|NotEqual(Enum) (Variables|Default|GetState) "NewEnumerator5")
    (if (> AxisValue 0.0)
      (Variables|Default|SetIsMovingRight true)
      (elif (< AxisValue 0.0)
        (Variables|Default|SetIsMovingRight false)))
    (Pawn|Input|AddMovementInput "1.000000, 0, 0" AxisValue false)))

(event Input|TouchEvents|InputTouch
  (params (Location :type Vector) (FingerIndex :type ETouchIndex%20Enum))
  ;[1 1 1] Handle Jump
  (:Pressed
    (Character|Jump)
    (Variables|Default|SetIsInAir true))
  (:Released
    (Character|StopJumping)))

(fn ConstructionScript)