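; Base actor for player bullets that damage enemies, with spawn and impact sounds.
; Each tick it moves along its local X axis at Speed scaled by delta time.
; On overlap it skips actors tagged IgnorePlayerBullet; otherwise it applies DamagePerHit to BP_EnemyBase targets with an impact sound, then destroys itself on any such hit.
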(event EventBeginPlay
  (Audio|PlaySound2D (Variables|Default|GetSoundOnSpawn) 0.6 1.0 0.0 0 0))

(event Collision|EventActorBeginOverlap
  (params (OtherActor :type Actor%20Object%20Reference))
  ;[1 1 1] Destruction
  (if (Utilities|IsValid OtherActor)
    (bind _output_get (Variables|Default|SetHitActor OtherActor))
    (if (not (Utilities|Array|ContainsItem (Variables|/Script/Engine.Actor|GetTags _output_get) "IgnorePlayerBullet"))
      ;[1 1 1] Enemy Takes Damage
      (bind _asbp_enemy_base (Utilities|Casting|CastToBP_EnemyBase (Variables|Default|GetHitActor))
        (:then
          (Default|TakeDamage _asbp_enemy_base (Variables|Default|GetDamagePerHit))
          (Utilities|IsValid (Variables|Default|GetSoundOnImpact)
            (:Is%20Valid
              (Audio|PlaySound2D (Variables|Default|GetSoundOnImpact) 5.0 1.0 0.0 0 0))
            (:Is%20Not%20Valid
              _)))
        (:CastFailed
          _))
      ;[1 1 1] Remove Bullet Actor
      (Actor|DestroyActor))))

(event EventTick
  (params (DeltaSeconds :type Float%20%28single-precision%29))
  (Transformation|AddActorLocalOffset (Math|Vector|MakeVector (* (Variables|Default|GetSpeed) 1.0 (Utilities|Time|GetWorldDeltaSeconds)) 0.0 0.0) false false))

(fn ConstructionScript)